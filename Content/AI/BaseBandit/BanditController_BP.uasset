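; AI controller for the base bandit enemy that reports pawn sightings to its Blackboard.
; PawnSensing's See Pawn event sets the player-spotted key and stores the seen pawn's location as last known, without checking that the pawn is the player.
; A short retriggerable delay clears the spotted flag once sightings stop, leaving the location intact.
; Tick does nothing, and AIPerception and debug-print nodes are disconnected leftovers.
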(event `self.ReceiveBeginPlay`)

(event `self.ReceiveTick`
  (params (DeltaSeconds :type "Float (single-precision)"))
  (if (`self.PlayerSpottedBool`)
    _))

(event `self.PawnSensing.OnSeePawn`
  (params (Pawn :type "Pawn Object Reference"))
  (bind _blackboardcomp (`self.BlackboardComp`))
  (bind _output_get (set `self.PlayerSpottedBool` true))
  (`BlackboardComponent.SetValueAsBool` _blackboardcomp (`self.PlayerSpottedKeyName`) _output_get)
  (`BlackboardComponent.SetValueAsVector` _blackboardcomp (`self.LastKnowLocationKeyName`) (`self.K2_GetActorLocation` Pawn))
  (`KismetSystemLibrary.RetriggerableDelay` 0.6)
  (bind _output_get_2 (set `self.PlayerSpottedBool` false))
  (`BlackboardComponent.SetValueAsBool` (`self.BlackboardComp`) (`self.PlayerSpottedKeyName`) _output_get_2))

(fn `UserConstructionScript`)