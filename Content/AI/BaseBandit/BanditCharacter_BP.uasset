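; Bandit AI enemy character built for reuse through activate and reset events, which set its active state.
; Activation restores health and starts the behavior tree.
; Fire, slow-mo and stun damage only print debug messages; other damage updates health by subtracting it from Damage (reversed operands).
; At zero or below, it disables collision, stops the tree, then after a delay teleports to its BeginPlay location and broadcasts death.
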(event `self.ReceiveBeginPlay`
  (set `self.DeadLocation` (`self.K2_GetActorLocation`)))

(event `/Game/AI/AI_Manager/Interfaces/IEnemies.ActivateEnemy`
  (set `self.isActive` true)
  (set `self.BanditHealth` (`self.MaxHealth`))
  (set `self.isDead` false)
  (`self.StartBehaviorTree`))

(event `/Game/AI/AI_Manager/Interfaces/IEnemies.ResetEnemy`
  (set `self.isActive` false))

(event `EnemyCanReset`
  (`KismetSystemLibrary.Delay` 1.0) ; Delay is needed as we are running a ragdoll perhaps? Later we will use some effect for explosion or something
  (`self.K2_SetActorLocation` (`self.DeadLocation`) false true)
  (`self.OnEnemyDead`))

(event `self.ReceiveAnyDamage`
  (params (Damage :type "Float (single-precision)") (DamageType :type "DamageType Object Reference") (InstigatedBy :type "Controller Object Reference") (DamageCauser :type "Actor Object Reference"))
  (if (== DamageType "/Game/AI/DamageTypes/FireAilment_DT.FireAilment_DT")
    (`KismetSystemLibrary.PrintString` "I'm on fire!" true true (struct :`R` 1.0 :`B` 0.007763 :`A` 1.0) 10.0)
    (elif (== DamageType "/Game/AI/DamageTypes/SlowMo_DT.SlowMo_DT_C")
      (`KismetSystemLibrary.PrintString` "I'm frozen!" true true (struct :`R` 1.0 :`B` 0.007763 :`A` 1.0) 10.0)
      (elif (== DamageType "/Game/AI/DamageTypes/Stun_DT.Stun_DT_C")
        (`KismetSystemLibrary.PrintString` "I'm on shocked!" true true (struct :`R` 1.0 :`B` 0.007763 :`A` 1.0) 10.0)
        (else
          (bind _output_get (set `self.BanditHealth` (- Damage (`self.BanditHealth`))))
          (if (<= _output_get 0.0)
            (`self.SetActorEnableCollision` false)
            (`self.StopBehaviorTree`)
            (`self.EnemyCanReset`)))))))

(fn `UserConstructionScript`)