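; Gib actor for the Ticker AI weapon, made up of six loose debris mesh pieces.
; On BeginPlay it enables physics simulation on all six gib meshes so they move as independent physics bodies.
; It has no other active logic: the construction script is empty and the overlap and tick events are disabled.
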(event `self.ReceiveActorBeginOverlap`
  (params (OtherActor :type "Actor Object Reference")))

(event `self.ReceiveBeginPlay`
  (`PrimitiveComponent.SetSimulatePhysics` (`self.GibMesh1`) true)
  (`PrimitiveComponent.SetSimulatePhysics` (`self.GibMesh2`) true)
  (`PrimitiveComponent.SetSimulatePhysics` (`self.GibMesh3`) true)
  (`PrimitiveComponent.SetSimulatePhysics` (`self.GibMesh4`) true)
  (`PrimitiveComponent.SetSimulatePhysics` (`self.GibMesh5`) true)
  (`PrimitiveComponent.SetSimulatePhysics` (`self.GibMesh6`) true))

(event `self.ReceiveTick`
  (params (DeltaSeconds :type "Float (single-precision)")))

(fn `UserConstructionScript`)