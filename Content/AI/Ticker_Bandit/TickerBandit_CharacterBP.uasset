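; Ticker Bandit enemy character that is activated and reset for reuse, running a behavior tree while alive.
; Activation restores health and starts the tree, while any damage lowers health, with debug prints for fire darts and Rock Punch.
; Rock Punch also launches the bandit along its own forward vector.
; At zero health it stops the tree, waits briefly, teleports to its BeginPlay location and broadcasts its death.
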(event `self.ReceiveBeginPlay`
  (set `self.DeadLocation` (`self.K2_GetActorLocation`)))

(event `/Game/AI/AI_Manager/Interfaces/IEnemies.ActivateEnemy`
  (set `self.isActive` true)
  (set `self.BanditHealth` (`self.MaxHealth`))
  (set `self.isDead` false)
  (`self.StartBehaviorTree`))

(event `/Game/AI/AI_Manager/Interfaces/IEnemies.ResetEnemy`
  (set `self.isActive` false))

(event `EnemyCanReset`
  (`KismetSystemLibrary.Delay` 1.0) ; Delay is needed as we are running a ragdoll perhaps? Later we will use some effect for explosion or something
  (`self.K2_SetActorLocation` (`self.DeadLocation`) false true)
  (`self.OnEnemyDead`))

(event `self.ReceiveAnyDamage`
  (params (Damage :type "Float (single-precision)") (DamageType :type "DamageType Object Reference") (InstigatedBy :type "Controller Object Reference") (DamageCauser :type "Actor Object Reference"))
  (cast `/Game/CharacterControls/Spells/MyFireDart` DamageCauser
    (:`then`
      (`KismetSystemLibrary.PrintString` "I'm on fire!" true true (struct :`R` 1.0 :`B` 0.007763 :`A` 1.0) 10.0)
      (bind _output_get (set `self.BanditHealth` (- (`self.BanditHealth`) Damage) :!label _label))
      (if (<= _output_get 0.0)
        (`self.StopBehaviorTree`)
        (`self.EnemyCanReset`)))
    (:`CastFailed`
      (cast `/Game/CharacterControls/Spells/RockPunch_BP` DamageCauser
        (:`then`
          (`KismetSystemLibrary.PrintString` "Im hit by Rock Punch!" true true (struct :`R` 1.0 :`B` 0.007763 :`A` 1.0) 10.0)
          (`self.LaunchCharacter` (* (`self.GetActorForwardVector`) (`self.RockPunchKnockback`)) true true)
          (goto _label))
        (:`CastFailed`
          (bind _output_get_2 (set `self.BanditHealth` (- (`self.BanditHealth`) Damage)))
          (if (<= _output_get_2 0.0)
            (`self.StopBehaviorTree`)
            (`self.EnemyCanReset`)))))))

(fn `UserConstructionScript`)