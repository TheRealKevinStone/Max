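; Enemy pattern actor that runs a reusable group of enemies placed as child actors, for use by the AI system.
; GetEnemiesInPattern caches each child actor and its starting location, then binds to every bandit's OnEnemyDead dispatcher.
; StartPattern activates all enemies by message and flags the pattern as spawned.
; When the death count covers the whole group, it broadcasts OnPatternEnded, resets the enemies and teleports them back for reuse.
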(event `self.ReceiveBeginPlay`)

(event `self.ReceiveActorBeginOverlap`
  (params (OtherActor :type "Actor Object Reference")))

(event `self.ReceiveTick`
  (params (DeltaSeconds :type "Float (single-precision)")))

(event `GetEnemiesInPattern`
  (`self.GetAllEnemies`) ; Populate all enemies array
  (for _array_element (`self.AllEnemies`)
    (bind _asbandit_character_bp (cast `/Game/AI/BaseBandit/BanditCharacter_BP` _array_element))
    (add `/Game/AI/BaseBandit/BanditCharacter_BP.OnEnemyDead` _asbandit_character_bp (delegate `OnEnemyDead`)) ; Bind to OnEnemyDead dispatcher so we will know when enemy dead
  ))

(event `OnEnemyDead`
  (set `self.DeadEnemiesCount` (+ (`self.DeadEnemiesCount`) 1)) ; Increase the count
  (if (`self.CheckIfPatternIsFinished`)
    (`self.OnPatternEnded`)
    (`self.EndPattern`)))

(fn `CheckIfPatternIsFinished`
  (returns (`All Enemies Dead` :type Boolean))
  (return (>= (`self.DeadEnemiesCount`) (`KismetArrayLibrary.Array_Length` (`self.AllEnemies`)))))

(fn `EndPattern`
  (for _array_element (`self.AllEnemies`)
    (message `/Game/AI/AI_Manager/Interfaces/IEnemies.ResetEnemy` _array_element) ; Call ResetEnemy on Bandit
  )
  (for (_array_element_2 _array_index) (`self.K2_GetComponentsByClass` "/Script/Engine.ChildActorComponent")
    (`self.K2_SetActorLocation` (`ChildActorComponent.ChildActor` _array_element_2) (`KismetArrayLibrary.Array_Get` (`self.AllEnemiesLocation`) _array_index) false true))
  (set `self.DeadEnemiesCount` 0) ; Reset dead count
)

(fn `GetAllEnemies`
  (for _array_element (`self.K2_GetComponentsByClass` "/Script/Engine.ChildActorComponent")
    (bind _childactor (`ChildActorComponent.ChildActor` _array_element))
    (`KismetArrayLibrary.Array_Add` (`self.AllEnemies`) _childactor)
    (`KismetArrayLibrary.Array_Add` (`self.AllEnemiesLocation`) (`self.K2_GetActorLocation` _childactor))))

(fn `Start Pattern`
  (for _array_element (`self.AllEnemies`)
    (message `/Game/AI/AI_Manager/Interfaces/IEnemies.ActivateEnemy` _array_element))
  (set `self.bWasSpawnedEarlier` true))

(fn `UserConstructionScript`)