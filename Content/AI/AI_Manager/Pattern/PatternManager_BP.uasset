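; Level manager that runs enemy patterns at the player's starting location until the level's time limit ends.
; It caches every Pattern_BP and its original location, then randomly picks an unused one whose difficulty nearly matches a curve sampled by level progress.
; If none match, it retries with a slightly wider tolerance up to a cap.
; Finished patterns teleport back to their original location, and the next starts after that pattern's custom delay.
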(event `self.ReceiveBeginPlay`
  (set `self.PatternStartLocation` (`self.K2_GetActorLocation` (`GameplayStatics.GetPlayerPawn` 0)))
  (`self.GetAllPatterns`)
  (`self.FindPattern`))

(event `self.ReceiveTick`
  (params (DeltaSeconds :type "Float (single-precision)"))
  ;[0.03627 0 1] It will make sure we stop when level time ended
  (if (`self.ManagerEnabled`)
    (bind _output_get (set `self.CurrentTime` (+ DeltaSeconds (`self.CurrentTime`))))
    (if (>= _output_get (`self.MaximumLevelTime`))
      (set `self.ManagerEnabled` false)
      (`self.OnLevelEndedWithTime`))))

(event `CurrentPatternEnded`
  (bind _allpatterns (`self.AllPatterns`))
  (bind _currentpattern (`self.CurrentPattern`))
  (bind _returnvalue (`KismetArrayLibrary.Array_Find` _allpatterns (`self.CurrentPattern`)))
  ;[0 0.08375 1] This will make sure current pattern wil move outside the screen and start another pattern after delay
  (`self.K2_SetActorLocation` (`KismetArrayLibrary.Array_Get` _allpatterns _returnvalue) (`KismetArrayLibrary.Array_Get` (`self.PatternsLocations`) _returnvalue) false true) ; Move current pattern to start location outside the view
  (remove `/Game/AI/AI_Manager/Pattern/Pattern_BP.OnPatternEnded` _currentpattern (delegate `CurrentPatternEnded`)) ; Always make sure you unbind an event. It will prevent crashes later on
  (`KismetSystemLibrary.Delay` (`/Game/AI/AI_Manager/Pattern/Pattern_BP.CustomDelayBeforeStart` _currentpattern))
  (`self.FindPattern`) ; Find Next Pattern
)

(event `FindPattern`
  ;[0.2096 1 0.08452] Finding the next pattern to run according to tolerance
  (if (`self.ManagerEnabled`)
    (bind _success_ (`self.TryToGetBestPatterns` (`self.CurrentTolerance`)))
    (if _success_
      (bind _output_get (set `self.CurrentPattern` (`KismetArrayLibrary.Array_Get` (`self.NextBestPattern`) (`KismetMathLibrary.RandomIntegerInRange` 0 (`KismetArrayLibrary.Array_LastIndex` (`self.NextBestPattern`)))))) ; Store active pattern
      (add `/Game/AI/AI_Manager/Pattern/Pattern_BP.OnPatternEnded` _output_get (delegate `CurrentPatternEnded`)) ; So Manager will know when pattern will end
      (`self.K2_SetActorLocation` (`self.CurrentPattern`) (`self.PatternStartLocation`) false false) ; Move pattern in front of the player
      (`/Game/AI/AI_Manager/Pattern/Pattern_BP.Start Pattern` (`self.CurrentPattern`))
      (else
        (set `self.CurrentTolerance` (+ (`self.CurrentTolerance`) 0.1)) ; increase tolerance
        (if (> (`self.CurrentTolerance`) 0.25)
          (`KismetSystemLibrary.PrintString` "CANT FIND PATTERN")
          (else
            (`self.FindPattern`) ; Try to find pattern again with a higher tolerance
          ))))))

(fn `GetAllPatterns`
  ;[1 1 1] Gett all patterns in level and add the locations of them in an array named Patterns Locations
  (bind _outactors (`GameplayStatics.GetAllActorsOfClass` "/Game/AI/AI_Manager/Pattern/Pattern_BP.Pattern_BP_C"))
  (for _array_element _outactors
    (`KismetArrayLibrary.Array_Add` (`self.AllPatterns`) _array_element)
    (`/Game/AI/AI_Manager/Pattern/Pattern_BP.GetEnemiesInPattern` _array_element)
    (`KismetArrayLibrary.Array_Add` (`self.PatternsLocations`) (`self.K2_GetActorLocation` _array_element))))

(fn `GetDifficultyFromCurve`
  (returns (Difficulty :type "Float (double-precision)"))
  (return (`CurveFloat.GetFloatValue` (`self.Difficulty`) (`self.GetLevelProgress`))))

(fn `GetLevelProgress`
  (returns (Progress :type "Float (double-precision)"))
  (return (/ (`self.CurrentTime`) (`self.MaximumLevelTime`))))

(fn `TryToGetBestPatterns`
  (params (Tolerance :type "Float (double-precision)"))
  (returns (`Success?` :type Boolean))
  ;[0 1 0.2411] This is basically searching for patterns that wasn’t enabled earlier and theirs difficulty is nearly equal than on curve.
  (`KismetArrayLibrary.Array_Clear` (`self.NextBestPattern`)) ; first clear the array
  (for _array_element (`self.AllPatterns`)
    (if (`/Game/AI/AI_Manager/Pattern/Pattern_BP.bWasSpawnedEarlier` _array_element)
      _
      (elif (`KismetMathLibrary.NearlyEqual_FloatFloat` (`/Game/AI/AI_Manager/Pattern/Pattern_BP.Difficulty` _array_element) (`self.GetDifficultyFromCurve`) Tolerance)
        (`KismetArrayLibrary.Array_Add` (`self.NextBestPattern`) _array_element)
        (set `self.FoundSomething?` true))))
  (return (`self.FoundSomething?`)))

(fn `UserConstructionScript`)