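; Pattern manager that runs enemy wave patterns once the player overlaps its trigger sphere.
; It picks a random unused Pattern_BP whose difficulty nearly matches a progress-based curve, widening tolerance until one fits.
; Level patterns are reused by teleporting them to random target points, then back to their original locations when they end, chaining the next.
; The level-timer logic is disconnected from Tick, so progress never advances here.
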(event `self.ReceiveBeginPlay`
  (bind _spawnlocations (`self.SpawnLocations`))
  ;[0.02254 1 0] Get Spawn Locations
  (bind _outactors (`GameplayStatics.GetAllActorsOfClass` "/Game/AI/TestTargetPoint_BP.TestTargetPoint_BP_C"))
  (for _array_element _outactors
    (`KismetArrayLibrary.Array_Add` _spawnlocations (`self.K2_GetActorLocation` _array_element))
    (set `self.PatternSpawnLocation` (`KismetArrayLibrary.Array_Get` _spawnlocations))))

(event `self.TriggerSphere.OnComponentBeginOverlap`
  (params (OtherActor :type "Actor Object Reference") (OtherComp :type "PrimitiveComponent Object Reference") (OtherBodyIndex :type Integer) (bFromSweep :type Boolean) (SweepResult :type "HitResult Structure (by ref)"))
  ;[1 0.7745 0] Activate Wave Pattern
  (if (== (`self.ManagerEnabled`) true)
    _
    (elif (== OtherActor (`GameplayStatics.GetPlayerPawn` 0))
      (`self.GetAllPatterns`)
      (`self.FindPattern`)
      (set `self.ManagerEnabled` true))))

(event `self.ReceiveTick`
  (params (DeltaSeconds :type "Float (single-precision)"))
  ;[0.03627 0 1] It will make sure we stop when level time ended
)

(event `CurrentPatternEnded`
  (bind _allpatterns (`self.AllPatterns`))
  (bind _currentpattern (`self.CurrentPattern`))
  (bind _returnvalue (`KismetArrayLibrary.Array_Find` _allpatterns (`self.CurrentPattern`)))
  ;[0 0.08375 1] This will make sure current pattern wil move outside the screen and start another pattern after delay
  (`self.K2_SetActorLocation` (`KismetArrayLibrary.Array_Get` _allpatterns _returnvalue) (`KismetArrayLibrary.Array_Get` (`self.PatternsLocations`) _returnvalue) false true) ; Move current pattern to start location outside the view
  (remove `/Game/AI/AI_Manager/Pattern_Classes/Pattern_BP.OnPatternEnded` _currentpattern (delegate `CurrentPatternEnded`)) ; Always make sure you unbind an event. It will prevent crashes later on
  (`KismetSystemLibrary.Delay` (`/Game/AI/AI_Manager/Pattern_Classes/Pattern_BP.CustomDelayBeforeStart` _currentpattern))
  (`self.FindPattern`) ; Find Next Pattern
)

(event `FindPattern`
  (bind _spawnlocations (`self.SpawnLocations`))
  ;[0.2096 1 0.08452] Finding the next pattern to run according to tolerance
  (bind _success_ (`self.TryToGetBestPatterns` (`self.CurrentTolerance`)))
  (`KismetSystemLibrary.Delay` 0.2)
  (if _success_
    (bind _output_get (set `self.CurrentPattern` (`KismetArrayLibrary.Array_Get` (`self.NextBestPattern`) (`KismetMathLibrary.RandomIntegerInRange` 0 (`KismetArrayLibrary.Array_LastIndex` (`self.NextBestPattern`)))))) ; Store active pattern
    (add `/Game/AI/AI_Manager/Pattern_Classes/Pattern_BP.OnPatternEnded` _output_get (delegate `CurrentPatternEnded`)) ; So Manager will know when pattern will end
    (`self.K2_SetActorLocation` (`self.CurrentPattern`) (`KismetArrayLibrary.Array_Get` _spawnlocations (`KismetMathLibrary.RandomIntegerInRange` 0 (`KismetArrayLibrary.Array_LastIndex` _spawnlocations))) false true) ; Move pattern to location
    (`/Game/AI/AI_Manager/Pattern_Classes/Pattern_BP.Start Pattern` (`self.CurrentPattern`))
    (else
      (set `self.CurrentTolerance` (+ (`self.CurrentTolerance`) 0.1)) ; increase tolerance
      (if (> (`self.CurrentTolerance`) 2.0)
        (`KismetSystemLibrary.PrintString` "CANT FIND PATTERN")
        (else
          (`self.FindPattern`) ; Try to find pattern again with a higher tolerance
        )))))

(fn `GetAllPatterns`
  ;[1 1 1] Gett all patterns in level and add the locations of them in an array named Patterns Locations
  (`KismetSystemLibrary.PrintString` "Starting Pattering...." true true (struct :`R` 0.139015 :`G` 0.515 :`B` 0.177146 :`A` 1.0) 5.0)
  (bind _outactors (`GameplayStatics.GetAllActorsOfClass` "/Game/AI/AI_Manager/Pattern_Classes/Pattern_BP.Pattern_BP_C"))
  (for _array_element _outactors
    (`KismetArrayLibrary.Array_Add` (`self.AllPatterns`) _array_element)
    (`/Game/AI/AI_Manager/Pattern_Classes/Pattern_BP.GetEnemiesInPattern` _array_element)
    (`KismetArrayLibrary.Array_Add` (`self.PatternsLocations`) (`self.K2_GetActorLocation` _array_element))))

(fn `GetDifficultyFromCurve`
  (returns (Difficulty :type "Float (double-precision)"))
  (return (`CurveFloat.GetFloatValue` (`self.Difficulty`) (`self.GetLevelProgress`))))

(fn `GetLevelProgress`
  (returns (Progress :type "Float (double-precision)"))
  (return (/ (`self.CurrentTime`) (`self.MaximumLevelTime`))))

(fn `Register Pattern Manager`
  ;[1 1 1] Register to Game state about the pattern so time can be kept track
  (bind _asfranco_game_state (cast `/Game/AI/AI_Manager/Franco_GameState` (`GameplayStatics.GetGameState`)))
  (`/Game/AI/AI_Manager/Franco_GameState.Set Pattern Manager` _asfranco_game_state self))

(fn `TryToGetBestPatterns`
  (params (Tolerance :type "Float (double-precision)"))
  (returns (`Success?` :type Boolean))
  (bind _nextbestpattern (`self.NextBestPattern`))
  ;[0 1 0.2411] This is basically searching for patterns that wasn’t enabled earlier and theirs difficulty is nearly equal than on curve.
  (`KismetArrayLibrary.Array_Clear` (`self.NextBestPattern`)) ; first clear the array
  (for _array_element (`self.AllPatterns`)
    (if (`/Game/AI/AI_Manager/Pattern_Classes/Pattern_BP.bWasSpawnedEarlier` _array_element)
      _
      (elif (`KismetMathLibrary.NearlyEqual_FloatFloat` (`/Game/AI/AI_Manager/Pattern_Classes/Pattern_BP.Difficulty` _array_element) (`self.GetDifficultyFromCurve`) Tolerance)
        (`KismetArrayLibrary.Array_Add` (`self.NextBestPattern`) _array_element)
        (set `self.FoundSomething?` true))))
  (return (`KismetArrayLibrary.Array_Contains` _nextbestpattern (`KismetArrayLibrary.Array_Get` _nextbestpattern (`KismetArrayLibrary.Array_LastIndex` _nextbestpattern)))))

(fn `UserConstructionScript`)